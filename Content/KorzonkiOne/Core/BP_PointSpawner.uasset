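; BP_PointSpawner is an actor that repeatedly spawns BP_PickupBase pickups at points marked by its scene components.
; BeginPlay collects the components, excluding the default root, and starts a delayed one-shot timer.
; SpawnPickup picks a random point, re-rolling while a sphere overlap finds a player character there.
; It then spawns the pickup with random yaw and sets another one-shot timer with a randomized delay.
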(event `self.ReceiveBeginPlay`
  (bind _output_get (set `self.Scenes` (`self.K2_GetComponentsByClass` "/Script/Engine.SceneComponent")))
  (`KismetArrayLibrary.Array_RemoveItem` _output_get (`self.DefaultSceneRoot`))
  (`KismetSystemLibrary.K2_SetTimerDelegate` (`|CreateDelegate` :!event `SpawnPickup`) 5.0))

(fn `SpawnPickup`
  (locals (SpawnLoc :type "Vector Structure") (NewSpawnLoc :type "Vector Structure"))
  (bind _scenes (`self.Scenes`))
  (bind _output_get (set `local.NewSpawnLoc` (`SceneComponent.K2_GetComponentLocation` (`|GetArrayItem` _scenes (`KismetMathLibrary.RandomIntegerInRange` 0 (- (`KismetArrayLibrary.Array_Length` _scenes) 1)))) :!label _label))
  (bind _outactors (`KismetSystemLibrary.SphereOverlapActors` _output_get 45.0 (`|MakeArray` "ObjectTypeQuery3" :!type "EObjectTypeQuery Enum") "/Game/KorzonkiOne/Core/BP_PlayerCharacter.BP_PlayerCharacter_C" (`|MakeArray` self :!type "Actor Object Reference")))
  (if (> (`KismetArrayLibrary.Array_Length` _outactors) 0)
    (goto _label)
    (else
      (`|SpawnActorFromClass` "/Game/KorzonkiOne/Core/Pickups/BP_PickupBase.BP_PickupBase_C" (`KismetMathLibrary.MakeTransform` (`local.NewSpawnLoc`) (`KismetMathLibrary.MakeRotator` 0.0 0.0 (`KismetMathLibrary.RandomFloatInRange` 0.0 360.0))) "Undefined" "OverrideRootScale" null null)
      (`KismetSystemLibrary.K2_SetTimerDelegate` (`|CreateDelegate` :!event `SpawnPickup`) (`KismetMathLibrary.RandomFloatInRange` 4.0 6.0)))))

(fn `UserConstructionScript`)