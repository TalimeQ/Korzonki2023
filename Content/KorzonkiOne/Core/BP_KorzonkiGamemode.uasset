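; BP_KorzonkiGamemode is a game mode that sets up local players and tracks player IDs.
; On BeginPlay it gets all active platform users and creates a player with its own controller for each one after the first.
; AssignPlayerId increments a counter and maps it to the given controller.
; GetPlayerData returns that controller's stored ID, or -1 when none exists.
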(event `self.ReceiveBeginPlay`
  (bind _outusers (`PlatformInputDeviceMapperLibrary.GetAllActiveUsers`))
  (for (_array_element _array_index) _outusers
    (bind _returnvalue (> _array_index 0))
    (if _returnvalue
      (`GameplayStatics.CreatePlayerFromPlatformUser` _array_element _returnvalue))))

(fn `AssignPlayerId`
  (params (Controller :type "PlayerController Object Reference"))
  (returns (PlayerId :type Integer))
  (`/Engine/EditorBlueprintResources/StandardMacros.IncrementInt` (`self.PlayerId`)
    (:`  `
      (`BlueprintMapLibrary.Map_Add` (`self.PlayerToID`) Controller (`self.PlayerId`))
      (return (`self.PlayerId`)))))

(fn `GetPlayerData`
  (params (Controller :type "PlayerController Object Reference"))
  (returns (NewParam :type Integer))
  (bind (_value _returnvalue) (`BlueprintMapLibrary.Map_Find` (`self.PlayerToID`) Controller))
  (if _returnvalue
    (return _value)
    (else
      (return -1))))

(fn `UserConstructionScript`)