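; Game state Blueprint for Korzonki that tracks each player's score and detects when a player wins.
; CreateScoreTrack registers a player in a score map at zero.
; Score adds to a controller's entry and fires OnScoreChanged, or prints a debug string if the controller is missing.
; VerifyScores then scans all entries and fires OnPlayerWon for each one at or above ScoreToWin.
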(event `self.ReceiveBeginPlay`)

(fn `CreateScoreTrack`
  (params (PlayerRef :type "PlayerController Object Reference"))
  (`BlueprintMapLibrary.Map_Add` (`self.Player Ref`) PlayerRef))

(fn `Score`
  (params (Controller :type "PlayerController Object Reference") (ScoreAmount :type Integer))
  (locals (CurrentScore :type Integer))
  (bind (_value _returnvalue) (`BlueprintMapLibrary.Map_Find` (`self.Player Ref`) Controller))
  (if _returnvalue
    (bind _output_get (set `local.CurrentScore` (+ _value (`local.ScoreAmount`))))
    (`BlueprintMapLibrary.Map_Add` (`self.Player Ref`) (`local.Controller`) _output_get)
    (`self.OnScoreChanged` (`local.CurrentScore`) (`local.Controller`))
    (`self.VerifyScores`)
    (else
      (`KismetSystemLibrary.PrintString` "JEBUO" true true (struct :`R` 1.0 :`B` 0.037247 :`A` 1.0)))))

(fn `UserConstructionScript`)

(fn `VerifyScores`
  (bind _keys (`BlueprintMapLibrary.Map_Keys` (`self.Player Ref`)))
  (for _array_element _keys
    (bind (_value _returnvalue) (`BlueprintMapLibrary.Map_Find` (`self.Player Ref`) _array_element))
    (if _returnvalue
      (if (>= _value (`self.ScoreToWin`))
        (`self.OnPlayerWon` _array_element)))))