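; BP_PickupBase is a score pickup actor, named as the base for pickups, that the player collects by touch.
; On BeginPlay it gives its Plane a random material from MaterialArray.
; When BP_PlayerCharacter overlaps its Box, it plays a 2D sound, calls Score on BP_KorzonkiGamestate to credit one point to that player's controller, then destroys itself.
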(event `self.ReceiveBeginPlay`
  (`PrimitiveComponent.SetMaterial` (`self.Plane`) 0 (`KismetArrayLibrary.Array_Random` (`self.MaterialArray`))))

(event `self.Box.OnComponentBeginOverlap`
  (params (OverlappedComponent :type "PrimitiveComponent Object Reference") (OtherActor :type "Actor Object Reference") (OtherComp :type "PrimitiveComponent Object Reference") (OtherBodyIndex :type Integer) (bFromSweep :type Boolean) (SweepResult :type "HitResult Structure (by ref)"))
  (bind _asbp_player_character (cast `/Game/KorzonkiOne/Core/BP_PlayerCharacter` OtherActor))
  (`GameplayStatics.SpawnSound2D` "/Game/KorzonkiOne/Music/up.up" 1.0 1.0 0.0 null)
  (`/Game/KorzonkiOne/Core/BP_KorzonkiGamestate.Score` (cast `/Game/KorzonkiOne/Core/BP_KorzonkiGamestate` (`GameplayStatics.GetGameState`) :!pure true) (cast `PlayerController` (`Pawn.GetController` _asbp_player_character) :!pure true) 1)
  (`self.K2_DestroyActor`))

(fn `UserConstructionScript`)