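; Player controller for Korzonki that sets up each player's input, pawn, camera and scoring at BeginPlay.
; It picks an Enhanced Input mapping context by controller ID; only the non-positive ID branch continues setup.
; That branch gets an ID from the gamemode, selects spawn and material, possesses a new character and views the BP_CameraPawn.
; It then creates a gamestate score track and claims the spawn's scoring zones.
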(event `self.ReceiveBeginPlay`
  (bind _returnvalue (subsystem `EnhancedInputLocalPlayerSubsystem`))
  (`KismetSystemLibrary.Delay` 0.0)
  (`/Engine/EditorBlueprintResources/StandardMacros.IsValid` _returnvalue
    (:`Is Valid`
      (if (> (`GameplayStatics.GetPlayerControllerID` null) 0)
        (`EnhancedInputSubsystemInterface.AddMappingContext` _returnvalue "/Game/ThirdPerson/Input/IMC_Default.IMC_Default" 0 (struct))
        (else
          (`EnhancedInputSubsystemInterface.AddMappingContext` _returnvalue "/Game/ThirdPerson/Input/IMC_Default2.IMC_Default2" 0 (struct))
          (bind _asbp_korzonki_gamemode (cast `/Game/KorzonkiOne/Core/BP_KorzonkiGamemode` (`GameplayStatics.GetGameMode`)))
          (bind _playerid (`/Game/KorzonkiOne/Core/BP_KorzonkiGamemode.AssignPlayerId` _asbp_korzonki_gamemode self))
          (bind _output_get (set `self.CurrentId` _playerid))
          (if (> _output_get 1)
            (bind _returnvalue_2 (`GameplayStatics.GetActorOfClass` "/Game/BP_Player2_Spawn.BP_Player2_Spawn_C"))
            (set `self.Spawn` _returnvalue_2)
            (set `self.SpawnTransform` (`self.GetTransform` _returnvalue_2))
            (set `self.Material` "/Game/KorzonkiOne/ArtAssets/Player/LudzikMat.LudzikMat")
            (else
              (bind _returnvalue_3 (`GameplayStatics.GetActorOfClass` "/Game/BP_PlayerSpawn.BP_PlayerSpawn_C"))
              (set `self.Spawn` _returnvalue_3)
              (set `self.SpawnTransform` (`self.GetTransform` _returnvalue_3))
              (set `self.Material` "/Game/KorzonkiOne/ArtAssets/Player/ludzik2_Mat.ludzik2_Mat")))
          (bind _returnvalue_4 (`|SpawnActorFromClass` "/Game/KorzonkiOne/Core/BP_PlayerCharacter.BP_PlayerCharacter_C" (`self.SpawnTransform`) "AlwaysSpawn" "OverrideRootScale" null null))
          (bind _output_get_2 (set `self.PlayerCharacter ` _returnvalue_4))
          (`PrimitiveComponent.SetMaterial` (`/Game/KorzonkiOne/Core/BP_PlayerCharacter.Plane` _output_get_2) 0 (`self.Material`))
          (`self.Possess` _output_get_2)
          (bind _returnvalue_5 (`GameplayStatics.GetActorOfClass` "/Game/KorzonkiOne/Core/BP_CameraPawn.BP_CameraPawn_C"))
          (`self.SetViewTargetWithBlend` _returnvalue_5)
          (bind _asbp_korzonki_gamestate (cast `/Game/KorzonkiOne/Core/BP_KorzonkiGamestate` (`GameplayStatics.GetGameState`)))
          (`/Game/KorzonkiOne/Core/BP_KorzonkiGamestate.CreateScoreTrack` _asbp_korzonki_gamestate self)
          (for _array_element (`/Game/BP_PlayerSpawnBase.PlayerScoringZones` (`self.Spawn`))
            (set `/Game/KorzonkiOne/Core/ScoringZone.OwningController` self _array_element)))))))

(fn `UserConstructionScript`)